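; BP_BotController is a bot controller that assigns itself to team 2 on BeginPlay and reports on what its AI perception sees.
; Each Tick it queries the AIPerceptionComponent's sight sense for known, perceived and currently perceived actors.
; It prints the three counts as one formatted debug line, using a fixed key.
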(event EventBeginPlay
  (Class|CoreAIController|SetTeamID 2))

(event EventTick
  (params (DeltaSeconds :type Float%20%28single-precision%29))
  (bind _aiperceptioncomponent (Variables|Default|GetAIPerceptionComponent))
  (Development|PrintText (Utilities|Text|FormatText "Known perc {a} 
Perceived {b} 
Currently {c}" (Utilities|Array|Length (Class|AIPerceptionComponent|GetKnownPerceivedActors _aiperceptioncomponent "/Script/AIModule.AISense_Sight")) (Utilities|Array|Length (Class|AIPerceptionComponent|GetPerceivedActors _aiperceptioncomponent "/Script/AIModule.AISense_Sight")) (Utilities|Array|Length (Class|AIPerceptionComponent|GetCurrentlyPerceivedActors _aiperceptioncomponent "/Script/AIModule.AISense_Sight"))) true true "(R=0.000000,G=0.660000,B=1.000000,A=1.000000)" 2.0 "No123ne"))

(fn ConstructionScript)